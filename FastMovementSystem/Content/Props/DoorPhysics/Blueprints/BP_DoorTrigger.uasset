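; BP_DoorTrigger is a sliding double door that opens when something overlaps its Trigger and closes when an overlap ends.
; The Open and Close events play and reverse one timeline, whose track slides the Left and Right panels in mirrored directions along local X from a fixed offset.
; Overlaps are neither filtered nor counted, so any exit starts closing the door.
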(event OnComponentBeginOverlap(Trigger)
  (params (OverlappedComponent :type Primitive%20Component%20Object%20Reference) (OtherActor :type Actor%20Object%20Reference) (OtherComp :type Primitive%20Component%20Object%20Reference) (OtherBodyIndex :type Integer) (bFromSweep :type Boolean) (SweepResult :type Hit%20Result%20Structure%20%28by%20ref%29))
  (CallFunction|Open))

(event OnComponentEndOverlap(Trigger)
  (params (OverlappedComponent :type Primitive%20Component%20Object%20Reference) (OtherActor :type Actor%20Object%20Reference) (OtherComp :type Primitive%20Component%20Object%20Reference) (OtherBodyIndex :type Integer))
  (CallFunction|Close))

(event Custom|Close
  (bind _track (Timeline|TL_Open Reverse)
    (:Update
      (Transformation|SetRelativeLocation (Variables|Default|GetRight) (Math|Vector|MakeVector (+ _track 1e+02) 0.0 0.0) false false)
      (Transformation|SetRelativeLocation (Variables|Default|GetLeft) (Math|Vector|MakeVector (- (* _track -1.0) 1e+02) 0.0 0.0) false false))))

(event Custom|Open
  (bind _track (Timeline|TL_Open Play)
    (:Update
      (Transformation|SetRelativeLocation (Variables|Default|GetRight) (Math|Vector|MakeVector (+ _track 1e+02) 0.0 0.0) false false)
      (Transformation|SetRelativeLocation (Variables|Default|GetLeft) (Math|Vector|MakeVector (- (* _track -1.0) 1e+02) 0.0 0.0) false false))))

(fn ConstructionScript)